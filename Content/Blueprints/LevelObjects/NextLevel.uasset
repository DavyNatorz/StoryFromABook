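; NextLevel is a level-transition trigger that turns the page of an animated book and then streams in Level_1.
; Any actor overlap sets the NextLevel flag, prints a debug string and finds the book actor by class.
; It starts a forward page turn on the book, waits a fixed delay matching the turn duration, then loads the level visible and without blocking.
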(event `self.ReceiveActorBeginOverlap`
  (params (OtherActor :type "Actor Object Reference"))
  (if true
    (set `self.NextLevel` true)
    (`KismetSystemLibrary.PrintString` "NextLevel_True")
    (bind _returnvalue (`GameplayStatics.GetActorOfClass` (`self.Animated Book`)))
    (bind _asbp_animated_book (cast `/Game/AnimatedBooks/Blueprints/BP_AnimatedBook` _returnvalue))
    (if (`self.NextLevel`)
      (`/Game/AnimatedBooks/Blueprints/BP_AnimatedBook.TurnThePage` _asbp_animated_book false 5.0)
      (`KismetSystemLibrary.Delay` 5.0)
      (`GameplayStatics.LoadStreamLevel` "Level_1" true))))

(fn `UserConstructionScript`)