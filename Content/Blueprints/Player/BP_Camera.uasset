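; Camera actor for tracking the player, with side-scroller deadzone follow logic left disconnected.
; BeginPlay only caches BP_Player_Old; FollowPlayer eases pitch and yaw toward it and re-calls itself via Delay, but nothing live here starts it.
; The construction script seeds axes from ActorToFollow and, without a fixed Z, sets yaw toward it.
; Deadzone helpers compute horizontal (world Y) and Z positions, but only unreachable nodes call them.
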(event `self.ReceiveBeginPlay`
  (bind _asbp_player_old (cast `/Game/Blueprints/Player/BP_Player_Old` (`GameplayStatics.GetPlayerCharacter` 0)))
  (set `self.Character Reference` _asbp_player_old))

(event `Follow Player`
  (bind (_returnvalue_roll _returnvalue_pitch _returnvalue_yaw) (`KismetMathLibrary.BreakRotator` (`KismetMathLibrary.RInterpTo` (`self.K2_GetActorRotation`) (`KismetMathLibrary.FindLookAtRotation` (`self.K2_GetActorLocation`) (`self.K2_GetActorLocation` (`self.Character Reference`))) (`GameplayStatics.GetWorldDeltaSeconds`) (`self.Camera Follow Speed`))))
  ;[1 1 1] Camera Follow Player
  (`self.K2_SetActorRotation` (`KismetMathLibrary.MakeRotator` 0.0 _returnvalue_pitch _returnvalue_yaw))
  (`KismetSystemLibrary.Delay` 0.001)
  (`self.Follow Player`))

(event `self.ReceiveTick`
  (params (DeltaSeconds :type "Float (single-precision)")))

(fn `Get New X Value`
  (returns (`New X Axis` :type "Float (double-precision)"))
  (bind (_returnvalue_x _returnvalue_y) (`KismetMathLibrary.BreakVector` (`self.K2_GetActorLocation`)))
  (bind (_returnvalue_x_2 _returnvalue_y_2) (`KismetMathLibrary.BreakVector` (`self.K2_GetActorLocation`)))
  (bind (_returnvalue_x_3 _returnvalue_y_3) (`KismetMathLibrary.BreakVector` (`self.K2_GetActorLocation` (`self.Actor To Follow`))))
  (bind (_returnvalue_x_4 _returnvalue_y_4) (`KismetMathLibrary.BreakVector` (`self.K2_GetActorLocation` (`self.Actor To Follow`))))
  (bind _returnvalue (- _returnvalue_y_4 (`self.X Axis Deadzone`)))
  (bind _returnvalue_2 (+ _returnvalue_y_3 (`self.X Axis Deadzone`)))
  (if (> _returnvalue _returnvalue_y_2)
    (return _returnvalue)
    (elif (< _returnvalue_2 _returnvalue_y)
      (return _returnvalue_2)
      (else
        (return (`self.Camera X Axis`))))))

(fn `Get New Z Value`
  (returns (`New Z Axis` :type "Float (double-precision)"))
  (bind (_returnvalue_x _returnvalue_y _returnvalue_z) (`KismetMathLibrary.BreakVector` (`self.K2_GetActorLocation`)))
  (bind (_returnvalue_x_2 _returnvalue_y_2 _returnvalue_z_2) (`KismetMathLibrary.BreakVector` (`self.K2_GetActorLocation`)))
  (bind (_returnvalue_x_3 _returnvalue_y_3 _returnvalue_z_3) (`KismetMathLibrary.BreakVector` (`self.K2_GetActorLocation` (`self.Actor To Follow`))))
  (bind (_returnvalue_x_4 _returnvalue_y_4 _returnvalue_z_4) (`KismetMathLibrary.BreakVector` (`self.K2_GetActorLocation` (`self.Actor To Follow`))))
  (bind _returnvalue (- _returnvalue_z_4 (`self.Z Axis Deadzone`)))
  (bind _returnvalue_2 (+ _returnvalue_z_3 (`self.Z Axis Deadzone`)))
  (if (!= (`self.Fixed Z Axis`) 0.0)
    (return (`self.Fixed Z Axis`))
    (elif (> _returnvalue _returnvalue_z_2)
      (return _returnvalue)
      (elif (< _returnvalue_2 _returnvalue_z)
        (return _returnvalue_2)
        (else
          (return (`self.Camera Z Axis`)))))))

(fn `UserConstructionScript`
  (bind _actor_to_follow (`self.Actor To Follow`))
  (bind (_returnvalue_x _returnvalue_y _returnvalue_z) (`KismetMathLibrary.BreakVector` (`self.K2_GetActorLocation` _actor_to_follow)))
  (bind (_returnvalue_roll _returnvalue_pitch _returnvalue_yaw) (`KismetMathLibrary.BreakRotator` (`KismetMathLibrary.FindLookAtRotation` (`self.K2_GetActorLocation`) (`self.K2_GetActorLocation` (`self.Actor To Follow`)))))
  (`/Engine/EditorBlueprintResources/StandardMacros.IsValid` _actor_to_follow
    (:`Is Valid`
      (set `self.Camera X Axis` _returnvalue_y)
      (if (not (!= (`self.Fixed Z Axis`) 0.0))
        (bind _output_get (set `self.Camera Z Axis` (+ _returnvalue_z (`self.Z Axis Deadzone`))))
        (`self.K2_SetActorRotation` (`KismetMathLibrary.MakeRotator` 0.0 0.0 _output_get))
        (`self.K2_SetActorRotation` (`KismetMathLibrary.MakeRotator` 0.0 0.0 _returnvalue_yaw))))))